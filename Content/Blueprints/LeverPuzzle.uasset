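; LeverPuzzle is a Lights Out-style puzzle over an array of levers, solved when every lever is on.
; On BeginPlay it binds to each lever's toggle event and randomizes their states, forcing at least one off.
; Toggling a lever calls ActivateByPuzzle on its immediate array neighbors, without wrapping at the ends, then checks for a solve.
; A solve prints a success message and reshuffles the puzzle after a short delay.
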(event Custom|OnLeverToggled
  (params (Lever :type Lever%20Object%20Reference))
  (bind _levers (Variables|Default|GetLevers))
  (bind _returnvalue (Utilities|Array|FindItem _levers Lever))
  (bind _returnvalue_2 (- _returnvalue 1))
  (bind _returnvalue_3 (+ _returnvalue 1))
  (Utilities|FlowControl|Sequence
    (:then_0
      ;[1 1 1] Puzzle Mechanic
      (if (>= _returnvalue_2 0)
        (Default|ActivatebyPuzzle (Utilities|Array|Get(acopy) (Variables|Default|GetLevers) _returnvalue_2)))
      (if (< _returnvalue_3 (Utilities|Array|Length (Variables|Default|GetLevers)))
        (Default|ActivatebyPuzzle (Utilities|Array|Get(acopy) (Variables|Default|GetLevers) _returnvalue_3))))
    (:then_1
      (bind _is_solved (CallFunction|CheckPuzzleSolved))
      (if _is_solved
        (Development|PrintString "You did it!")
        (Utilities|FlowControl|Delay 2.0)
        (CallFunction|RandomizePuzzle)))))

(event EventBeginPlay
  (for _array_element (Variables|Default|GetLevers)
    (EventDispatchers|BindEventtoToggledEvent _array_element (delegate Custom|OnLeverToggled)))
  (CallFunction|RandomizePuzzle))

(fn ConstructionScript)

(fn CheckPuzzleSolved
  (for _array_element (Variables|Default|GetLevers)
    (if (not (Variables|/Game/Blueprints/Lever.Lever_C|GetIsOn _array_element))
      (return false)))
  (return true))

(fn RandomizePuzzle
  (bind _levers (Variables|Default|GetLevers))
  (for _array_element _levers
    (if (Math|Random|RandomBool)
      (Default|Flipon _array_element)
      (else
        (Default|FlipOff _array_element))))
  ;[1 1 1] Make sure at least one lever is off.
  (Default|FlipOff (Utilities|Array|Get(acopy) _levers (Math|Random|RandomInteger (- (Utilities|Array|Length _levers) 1)))))
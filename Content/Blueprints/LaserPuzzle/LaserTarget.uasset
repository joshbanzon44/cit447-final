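; Laser puzzle target that lights up in the color of the laser hitting it.
; LaserBounce stores the hit response as Active and passes the laser's color to PuzzleSolved, with no color matching.
; PuzzleSolved creates a new dynamic BatteryMat instance on SMParent each call, setting a bright laser-colored glow when active or a dark zero-intensity state otherwise.
; It also shows or hides Widget to match Active.
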(event EventBeginPlay)

(event Collision|EventActorBeginOverlap
  (params (OtherActor :type Actor%20Object%20Reference)))

(event EventTick
  (params (DeltaSeconds :type Float%20%28single-precision%29)))

(fn ConstructionScript
  (|CallParentFunction))

(fn PuzzleSolved
  (params (Color%20Laser :type Linear%20Color%20Structure))
  (bind _returnvalue (Rendering|Material|CreateDynamicMaterialInstance (Variables|Default|GetSM_Parent) 0 "/Game/Blueprints/LaserPuzzle/BatteryMat.BatteryMat" "None" :!class /Script/Engine.PrimitiveComponent))
  (Rendering|Material|SetScalarParameterValue _returnvalue "Intensity" (select (Variables|Default|GetActive) 2e+01 0.0) :!class /Script/Engine.MaterialInstanceDynamic)
  (Rendering|Material|SetVectorParameterValue _returnvalue "Color" (Math|Color|SelectColor Color%20Laser "(R=0.151042,G=0.049572,B=0.000000,A=1.000000)" (Variables|Default|GetActive)) :!class /Script/Engine.MaterialInstanceDynamic)
  (if (Variables|Default|GetActive)
    (Rendering|SetVisibility (Variables|Default|GetWidget) true false)
    (else
      (Rendering|SetVisibility (Variables|Default|GetWidget) false false))))

(fn LaserBounce
  (params (LaserHit :type Laser%20Object%20Reference) (HitResponse :type Boolean) (HitInfo :type Hit%20Result%20Structure))
  (Variables|Default|SetActive HitResponse)
  (CallFunction|PuzzleSolved (Variables|/Game/Blueprints/LaserPuzzle/LaserParent.LaserParent_C|GetLaserColor LaserHit))
  (return 0))
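; A laser puzzle reset button that returns the puzzle's reflectors to their starting transforms when activated.
; On BeginPlay it caches the location, raised along Z, and rotation of each actor in LaserReflects, and labels its widget "Reset Puzzle".
; Activate reapplies the cached transforms to each reflector's SMParent component.
; Hover and UnHover toggle custom depth rendering on the button meshes for highlighting.
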(event EventBeginPlay
  (for _array_element (Variables|Default|GetLaserReflects)
    (Utilities|Array|Add (Variables|Default|GetReflectLocations) (+ (Transformation|GetActorLocation _array_element) "0.000000,0.000000,200.000000"))
    (Utilities|Array|Add (Variables|Default|GetReflectRotations) (Transformation|GetActorRotation _array_element))
    (bind _asbasic_widget (Utilities|Casting|CastToBasicWidget (UserInterface|GetWidget (Variables|Default|GetWidget))))
    (Variables|/Script/UMG.TextBlock|SetText (Variables|/Game/UI/BasicWidget.BasicWidget_C|GetWidgetText _asbasic_widget) "Reset Puzzle")))

(event EventActivate
  (for (_array_element _array_index) (Variables|Default|GetLaserReflects)
    (Transformation|SetWorldLocationAndRotation (Variables|/Game/Blueprints/LaserPuzzle/LaserParent.LaserParent_C|GetSM_Parent _array_element) (Utilities|Array|Get(acopy) (Variables|Default|GetReflectLocations) _array_index) (Utilities|Array|Get(acopy) (Variables|Default|GetReflectRotations) _array_index) false false)))

(event EventHover
  (Rendering|SetRenderCustomDepth (Variables|Default|GetButton) true))

(event EventUnHover
  (Rendering|SetRenderCustomDepth (Variables|Default|GetStaticMesh) false))

(fn ConstructionScript)
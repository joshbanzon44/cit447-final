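; Laser beam actor for a laser puzzle, tinted by a dynamic material.
; Each tick, a box trace along its up vector stretches the mesh to the hit or full range.
; Target changes are signaled through LaserInterface and the spawner's following-laser removal, and hit actors return a bounce laser that is re-aimed while on a LaserReflect.
; CancelTargetHit releases or deactivates the last target and destroys the beam unless overridden.
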(event EventBeginPlay
  (CallFunction|ChangeColor))

(event EventTick
  (params (DeltaSeconds :type Float%20%28single-precision%29))
  (CallFunction|SetEndpoint))

(fn ConstructionScript
  (|CallParentFunction))

(fn ChangeColor
  (bind _returnvalue (Rendering|Material|CreateDynamicMaterialInstance (Variables|Default|GetSM_Parent) 0 "/Game/Blueprints/LaserPuzzle/LaserMat.LaserMat" "None" :!class /Script/Engine.PrimitiveComponent))
  (Rendering|Material|SetVectorParameterValue _returnvalue "Color" (Variables|Default|GetLaserColor) :!class /Script/Engine.MaterialInstanceDynamic))

(fn SetEndpoint
  (bind _returnvalue (Transformation|GetActorLocation))
  (bind _returnvalue_2 (Transformation|GetActorUpVector))
  (bind _returnvalue_3 (* _returnvalue_2 2.0))
  (bind _returnvalue_4 (+ _returnvalue _returnvalue_3))
  (bind _outhit (Collision|BoxTraceByChannel _returnvalue_4 (+ _returnvalue_4 (* _returnvalue_2 (LocalVariables|GetRange))) "0.500000,0.500000,0.500000" "0, 0, 0" "TraceTypeQuery1" false 0 "None"))
  (bind _output_get (LocalVariables|SetHit%20Info _outhit))
  (LocalVariables|SetHitActor (.HitActor (Collision|BreakHitResult _output_get)))
  (Transformation|SetWorldScale3D (Variables|Default|GetSM_Parent) (Math|Vector|MakeVector 0.05 0.05 (Math|Float|SelectFloat (/ (+ (.Distance (Collision|BreakHitResult _output_get)) 1.0) 1e+02) (/ (LocalVariables|GetRange) 1e+02) (.bBlockingHit (Collision|BreakHitResult _output_get)))))
  (LocalVariables|GetHitActor
    (:then
      (Utilities|FlowControl|Sequence
        (:then_0
          (if (== (Variables|Default|GetLastHitActor) (LocalVariables|GetHitActor))
            (bind _aslaser_reflect (Utilities|Casting|CastToLaserReflect (Variables|Default|GetLastHitActor)))
            (Transformation|SetActorLocation (Variables|Default|GetBounceLaser) (.ImpactPoint (Collision|BreakHitResult (LocalVariables|GetHit%20Info))) false false)
            (Transformation|SetActorRotation (Variables|Default|GetBounceLaser) (Default|CalculateRotation _aslaser_reflect (.ImpactPoint (Collision|BreakHitResult (LocalVariables|GetHit%20Info))) (.Normal (Collision|BreakHitResult (LocalVariables|GetHit%20Info))) (.TraceStart (Collision|BreakHitResult (LocalVariables|GetHit%20Info)))))
            (else
              (Utilities|FlowControl|Sequence
                (:then_0
                  (if (Utilities|DoesObjectImplementInterface (Variables|Default|GetLastHitActor) "/Game/Blueprints/LaserPuzzle/LaserInterface.LaserInterface_C")
                    (Default|RemoveFollowingLasers (Variables|Default|GetSpawnReference) self)))
                (:then_1
                  (if (Utilities|DoesObjectImplementInterface (LocalVariables|GetHitActor) "/Game/Blueprints/LaserPuzzle/LaserInterface.LaserInterface_C")
                    (bind _new_laser (Class|LaserInterface|LaserBounce(Message) (LocalVariables|GetHitActor) self true (LocalVariables|GetHit%20Info)))
                    (Variables|Default|SetBounceLaser _new_laser)))))))
        (:then_1
          (Variables|Default|SetLastHitActor (LocalVariables|GetHitActor)))))
    (:else
      (Utilities|FlowControl|Sequence
        (:then_0
          (bind _lasthitactor (Variables|Default|GetLastHitActor)
            (:then
              (if (Utilities|DoesObjectImplementInterface _lasthitactor "/Game/Blueprints/LaserPuzzle/LaserInterface.LaserInterface_C")
                (Class|LaserInterface|LaserBounce(Message) (Variables|Default|GetLastHitActor) self false (LocalVariables|GetHit%20Info))))
            (:else)))
        (:then_1
          (Variables|Default|SetLastHitActor 0)
          (Variables|Default|SetBounceLaser 0))))))

(fn UpdateID
  (params (Append :type String))
  (return (Utilities|String|Append (Variables|Default|GetLaserID) Append)))

(fn CancelTargetHit
  (params (Override :type Boolean))
  (Utilities|FlowControl|Sequence
    (:then_0
      (bind _lasthitactor (Variables|Default|GetLastHitActor)
        (:then
          (bind _aslaser_parent (Utilities|Casting|CastToLaserParent _lasthitactor))
          (if (and (Utilities|DoesObjectImplementInterface _aslaser_parent "/Game/Blueprints/LaserPuzzle/LaserInterface.LaserInterface_C") (Utilities|Array|IsEmpty (Variables|/Game/Blueprints/LaserPuzzle/LaserParent.LaserParent_C|GetLasersAttached _aslaser_parent)))
            (Class|LaserInterface|LaserBounce(Message) (Variables|Default|GetLastHitActor) self false)
            (else
              (Variables|/Game/Blueprints/LaserPuzzle/LaserParent.LaserParent_C|SetActive _aslaser_parent false))))
        (:else)))
    (:then_1
      (if Override
        (return false)
        (else
          (Actor|DestroyActor)
          (return true))))))
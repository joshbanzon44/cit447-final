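; LaserReflect is a laser puzzle reflector that bounces incoming lasers off its surface.
; On a hit, LaserBounce spawns a same-colored Laser at the impact point, its Z axis along the incoming direction mirrored by the surface normal.
; The bounce gets an updated ID and registers in LasersAttached and the spawn reference's ChildLasers.
; Without a hit response, a reverse loop destroys attached lasers whose IDs contain the incoming laser's ID.
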(event EventBeginPlay
  (|CallParentFunction) ; This node is disabled and will not be called.\nDrag off pins to build functionality.
)

(event Collision|EventActorBeginOverlap
  (params (OtherActor :type Actor%20Object%20Reference))
  (|CallParentFunction OtherActor) ; This node is disabled and will not be called.\nDrag off pins to build functionality.
)

(event EventTick
  (params (DeltaSeconds :type Float%20%28single-precision%29))
  (|CallParentFunction DeltaSeconds) ; This node is disabled and will not be called.\nDrag off pins to build functionality.
)

(fn ConstructionScript
  (|CallParentFunction))

(fn ClearAttachedLasers
  (params (ID%20Clear :type String))
  (bind _arrayelement (Utilities|Array|ReverseforEachLoop (Variables|Default|GetLasersAttached))
    (:LoopBody
      (Utilities|IsValid _arrayelement
        (:Is%20Valid
          (if (Utilities|String|Contains (Variables|/Game/Blueprints/LaserPuzzle/Laser.Laser_C|GetLaserID _arrayelement) ID%20Clear)
            (Actor|DestroyActor _arrayelement)
            (Utilities|Array|RemoveItem (Variables|Default|GetLasersAttached) _arrayelement)))))))

(fn CalculateRotation
  (params (Impact%20Point :type Vector) (Impact%20Normal :type Vector) (Trace%20Start :type Vector))
  (return (Math|Rotator|MakeRotfromZ (Math|Vector|MirrorVectorbyNormal (- Impact%20Point Trace%20Start) Impact%20Normal))))

(fn LaserBounce
  (params (LaserHit :type Laser%20Object%20Reference) (HitResponse :type Boolean) (HitInfo :type Hit%20Result%20Structure))
  (bind (_bblockinghit _binitialoverlap _time _distance _location _impactpoint _normal _impactnormal _physmat _hitactor _hitcomponent _hitbonename _bonename _hititem _elementindex _faceindex _tracestart) (Collision|BreakHitResult HitInfo))
  (if HitResponse
    (bind _returnvalue (Game|SpawnActorfromClass "/Game/Blueprints/LaserPuzzle/Laser.Laser_C" (Math|Transform|MakeTransform _impactpoint (CallFunction|CalculateRotation _impactpoint _impactnormal _tracestart) "1.000000,1.000000,1.000000") "Undefined" "MultiplyWithRoot" 0 (Default|UpdateID LaserHit "B") (Variables|/Game/Blueprints/LaserPuzzle/LaserParent.LaserParent_C|GetLaserColor LaserHit) (Variables|/Game/Blueprints/LaserPuzzle/LaserParent.LaserParent_C|GetSpawnReference LaserHit) 0))
    (Utilities|Array|Add (Variables|Default|GetLasersAttached) _returnvalue)
    (Utilities|Array|Add (Variables|/Game/Blueprints/LaserPuzzle/LaserSpawn.LaserSpawn_C|GetChild%20Lasers (Variables|/Game/Blueprints/LaserPuzzle/LaserParent.LaserParent_C|GetSpawnReference LaserHit)) _returnvalue)
    (return _returnvalue)
    (else
      (CallFunction|ClearAttachedLasers (Variables|/Game/Blueprints/LaserPuzzle/Laser.Laser_C|GetLaserID LaserHit)))))
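; Interactable lever that toggles between on and off, with hover highlighting through custom depth on its base and handle.
; Activate flips IsOn, plays or reverses a timeline that lerps the handle between two rotations, then calls the toggled event.
; ActivateByPuzzle, FlipOn and FlipOff drive the same flip without calling that event.
; The construction script poses the handle to match its initial IsOn state.
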(event Custom|ActivateByPuzzle
  (if (Variables|Default|GetIsOn)
    (Variables|Default|SetIsOn false)
    (bind _onoffpercent (Timeline|LeverRotation Reverse)
      (:Update
        (Transformation|SetRelativeRotation (Variables|Default|GetLever) (Math|Rotator|Lerp(Rotator) (Variables|Default|GetOffRotation) (Variables|Default|GetOnRotation) _onoffpercent) false false)))
    (else
      (Variables|Default|SetIsOn true)
      (Timeline|LeverRotation Play))))

(event Custom|FlipOff
  (if (Variables|Default|GetIsOn)
    (Variables|Default|SetIsOn false)
    (bind _onoffpercent (Timeline|LeverRotation Reverse)
      (:Update
        (Transformation|SetRelativeRotation (Variables|Default|GetLever) (Math|Rotator|Lerp(Rotator) (Variables|Default|GetOffRotation) (Variables|Default|GetOnRotation) _onoffpercent) false false)))))

(event Custom|FlipOn
  (if (not (Variables|Default|GetIsOn))
    (Variables|Default|SetIsOn true)
    (bind _onoffpercent (Timeline|LeverRotation Play)
      (:Update
        (Transformation|SetRelativeRotation (Variables|Default|GetLever) (Math|Rotator|Lerp(Rotator) (Variables|Default|GetOffRotation) (Variables|Default|GetOnRotation) _onoffpercent) false false)))))

(event EventBeginPlay
  (bind _onoffpercent (Timeline|LeverRotation SetNewTime)
    (:Update
      (Transformation|SetRelativeRotation (Variables|Default|GetLever) (Math|Rotator|Lerp(Rotator) (Variables|Default|GetOffRotation) (Variables|Default|GetOnRotation) _onoffpercent) false false))))

(event EventHover
  (Rendering|SetRenderCustomDepth (Variables|Default|GetBase) true)
  (Rendering|SetRenderCustomDepth (Variables|Default|GetLever) true))

(event EventUnHover
  (Rendering|SetRenderCustomDepth (Variables|Default|GetBase) false)
  (Rendering|SetRenderCustomDepth (Variables|Default|GetLever) false))

(event EventActivate
  (Utilities|FlowControl|Sequence
    (:then_0
      (if (Variables|Default|GetIsOn)
        (Variables|Default|SetIsOn false)
        (bind _onoffpercent (Timeline|LeverRotation Reverse)
          (:Update
            (Transformation|SetRelativeRotation (Variables|Default|GetLever) (Math|Rotator|Lerp(Rotator) (Variables|Default|GetOffRotation) (Variables|Default|GetOnRotation) _onoffpercent) false false)))
        (else
          (Variables|Default|SetIsOn true)
          (Timeline|LeverRotation Play))))
    (:then_1
      (Default|CallToggledEvent self))))

(fn ConstructionScript
  (Transformation|SetRelativeRotation (Variables|Default|GetLever) (select (Variables|Default|GetIsOn) (Variables|Default|GetOnRotation) (Variables|Default|GetOffRotation)) false false))
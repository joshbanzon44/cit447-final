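; BP_DirtyObjectManager tracks a set of dirty objects and unlocks a door once all of them are cleaned.
; On BeginPlay it binds to each object's VertexPaintable fully-cleaned delegate, then rescans the whole array whenever one fires.
; When none remain dirty, it shows a congratulations widget and opens the referenced door.
; Otherwise it prints a progress message and resets its IsAreaClean flag for the next check.
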(event Custom|OnObjectCleaned
  (for _array_element (Variables|Default|GetDirtyObjectsArray)
    (if (not (Variables|/Game/Blueprints/Cleaning/BP_BaseDirtyObject.BP_BaseDirtyObject_C|GetIsClean _array_element))
      (Variables|Default|SetIsAreaClean false)))
  (if (Variables|Default|GetIsAreaClean)
    (CallFunction|AreaCleaned)
    (else
      (Development|PrintString "another object cleaned, area not finished")
      (Variables|Default|SetIsAreaClean true))))

(event Custom|AreaCleaned
  (bind _returnvalue (UserInterface|CreateWidget "/Game/UI/BasicWidget.BasicWidget_C"))
  (Default|SetText _returnvalue "You have cleaned everything! 
Congratulations! The door is unlocked!")
  (UserInterface|Viewport|AddtoViewport _returnvalue 0)
  (Default|OpenDoor (Variables|Default|GetDoorRef)))

(event EventBeginPlay
  (for _array_element (Variables|Default|GetDirtyObjectsArray)
    (EventDispatchers|BindEventtoOnFullyCleanedDelegate (Variables|/Game/Blueprints/Cleaning/BP_BaseDirtyObject.BP_BaseDirtyObject_C|GetVertexPaintable _array_element) (delegate Custom|OnObjectCleaned))))

(fn ConstructionScript)
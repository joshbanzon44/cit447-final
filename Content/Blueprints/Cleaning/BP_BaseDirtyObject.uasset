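; Base actor for a cleanable dirty object that rewards the player with XP when fully cleaned.
; A VertexPaintable component supplies the clean percentage to a progress bar widget, which yaws toward the player and shows only while hovered.
; On full clean it flags itself clean, turns the bar green, enables custom depth on the mesh and sets Specular on a dynamic material created in the construction script.
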(event OnFullyCleanedDelegate(VertexPaintable)
  (Variables|Default|SetIsClean true)
  (CallFunction|UpdateWidget)
  (Rendering|SetRenderCustomDepth (Variables|Default|GetStaticMesh) true)
  (Rendering|Material|SetScalarParameterValue (Variables|Default|GetDynMat) "Specular" 0.1 :!class /Script/Engine.MaterialInstanceDynamic)
  (bind _asfirst_person_player_pawn (Utilities|Casting|CastToFirstPersonPlayerPawn (Game|GetPlayerCharacter 0)))
  (Class|StatsComponent|AddXP (Variables|/Game/Blueprints/Player/FirstPersonPlayerPawn.FirstPersonPlayerPawn_C|GetStatsComponent _asfirst_person_player_pawn) (Variables|Default|GetCompletedXP)))

(event EventBeginPlay
  (CallFunction|UpdateWidget)
  (Rendering|SetVisibility (Variables|Default|GetWidget) false false))

(event Collision|EventActorBeginOverlap
  (params (OtherActor :type Actor%20Object%20Reference)))

(event EventTick
  (params (DeltaSeconds :type Float%20%28single-precision%29))
  (Transformation|SetWorldRotation (Variables|Default|GetWidget) (Math|Rotator|MakeRotator 0.0 0.0 (.yaw (Math|Rotator|FindLookatRotation (Transformation|GetWorldLocation (Variables|Default|GetWidget)) (Transformation|GetActorLocation (Game|GetPlayerCharacter 0))))) false false))

(event EventHover
  (Rendering|SetVisibility (Variables|Default|GetWidget) true false))

(event EventUnHover
  (Rendering|SetVisibility (Variables|Default|GetWidget) false false))

(fn ConstructionScript
  (bind _staticmesh (Variables|Default|GetStaticMesh))
  (bind _returnvalue (Rendering|Material|CreateDynamicMaterialInstance _staticmesh 0 (Rendering|Material|GetMaterial _staticmesh 0) "None" :!class /Script/Engine.PrimitiveComponent))
  (Variables|Default|SetDynMat _returnvalue))

(fn UpdateWidget
  (bind _vertexpaintable (Variables|Default|GetVertexPaintable))
  (bind _percentclean (Variables|/Script/A4.VertexPaintableComponent|GetPercentClean _vertexpaintable))
  (bind _asprogress_bar (Utilities|Casting|CastToProgressBar (UserInterface|GetWidget (Variables|Default|GetWidget))))
  (Progress|SetPercent (Variables|/Game/UI/ProgressBar.ProgressBar_C|GetProgressBar _asprogress_bar) _percentclean)
  (if (>= _percentclean 1.0)
    (Variables|/Script/UMG.ProgressBar|SetFillColorAndOpacity (Variables|/Game/UI/ProgressBar.ProgressBar_C|GetProgressBar _asprogress_bar) "(R=0.000000,G=1.000000,B=0.000000,A=1.000000)")))
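; Shop actor where the player buys an apple or a diamond by walking into the matching collision volume.
; On overlap by a FirstPersonPlayerPawn with enough Money, it deducts the fixed price and spawns the item's NPC class at that item's spawn point.
; Otherwise both paths share a branch that shows a not-enough-money message, then resets it after a delay.
; SetLabels fills the shop's widget components with title, prices and buy prompts.
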(event Custom|OnComponentBeginOverlap_Event
  (params (OverlappedComponent :type Primitive%20Component%20Object%20Reference) (OtherActor :type Actor%20Object%20Reference) (OtherComp :type Primitive%20Component%20Object%20Reference) (OtherBodyIndex :type Integer) (bFromSweep :type Boolean) (SweepResult :type Hit%20Result%20Structure%20%28by%20ref%29))
  (bind _asfirst_person_player_pawn (Utilities|Casting|CastToFirstPersonPlayerPawn OtherActor))
  (if (>= (Variables|/Game/Blueprints/Player/FirstPersonPlayerPawn.FirstPersonPlayerPawn_C|GetMoney _asfirst_person_player_pawn) 100)
    (Default|ChangeMoney _asfirst_person_player_pawn -100)
    (Game|SpawnActorfromClass "/Game/Blueprints/NPCs/NPC_Diamond.NPC_Diamond_C" (Math|Transform|MakeTransform (Transformation|GetWorldLocation (Variables|Default|GetDiamondSpawn)) "0, 0, 0" "1.000000,1.000000,1.000000") "Undefined" "MultiplyWithRoot" 0 0)
    (else
      (bind _asbasic_widget (Utilities|Casting|CastToBasicWidget (UserInterface|GetWidget (Variables|Default|GetNomoney))))
      (Variables|/Script/UMG.TextBlock|SetText (Variables|/Game/UI/BasicWidget.BasicWidget_C|GetWidgetText _asbasic_widget) "Not 
enough 
money!")
      (Utilities|FlowControl|Delay 3.0)
      (CallFunction|SetLabels))))

(event Custom|OnComponentBeginOverlap_Event_0
  (params (OverlappedComponent :type Primitive%20Component%20Object%20Reference) (OtherActor :type Actor%20Object%20Reference) (OtherComp :type Primitive%20Component%20Object%20Reference) (OtherBodyIndex :type Integer) (bFromSweep :type Boolean) (SweepResult :type Hit%20Result%20Structure%20%28by%20ref%29))
  (bind _asfirst_person_player_pawn (Utilities|Casting|CastToFirstPersonPlayerPawn OtherActor))
  (if (>= (Variables|/Game/Blueprints/Player/FirstPersonPlayerPawn.FirstPersonPlayerPawn_C|GetMoney _asfirst_person_player_pawn) 50)
    (Default|ChangeMoney _asfirst_person_player_pawn -50)
    (Game|SpawnActorfromClass "/Game/Blueprints/NPCs/NPC_Apple.NPC_Apple_C" (Math|Transform|MakeTransform (Transformation|GetWorldLocation (Variables|Default|GetAppleSpawn)) "0, 0, 0" "1.000000,1.000000,1.000000") "Undefined" "MultiplyWithRoot" 0 0)
    (else
      (bind _asbasic_widget (Utilities|Casting|CastToBasicWidget (UserInterface|GetWidget (Variables|Default|GetNomoney))))
      (Variables|/Script/UMG.TextBlock|SetText (Variables|/Game/UI/BasicWidget.BasicWidget_C|GetWidgetText _asbasic_widget) "Not 
enough 
money!")
      (Utilities|FlowControl|Delay 3.0)
      (CallFunction|SetLabels))))

(event EventBeginPlay
  (CallFunction|SetLabels)
  (Collision|AssignOnComponentBeginOverlap (Variables|Default|GetDiamondCollision) (delegate Custom|OnComponentBeginOverlap_Event))
  (Collision|AssignOnComponentBeginOverlap (Variables|Default|GetAppleCollision) (delegate Custom|OnComponentBeginOverlap_Event_0)))

(fn ConstructionScript)

(fn SetLabels
  (bind _asbasic_widget (Utilities|Casting|CastToBasicWidget (UserInterface|GetWidget (Variables|Default|GetLabel))))
  (Variables|/Script/UMG.TextBlock|SetText (Variables|/Game/UI/BasicWidget.BasicWidget_C|GetWidgetText _asbasic_widget) "Apple and Diamond Shop")
  (bind _asbasic_widget_2 (Utilities|Casting|CastToBasicWidget (UserInterface|GetWidget (Variables|Default|GetPrice))))
  (Variables|/Script/UMG.TextBlock|SetText (Variables|/Game/UI/BasicWidget.BasicWidget_C|GetWidgetText _asbasic_widget_2) "Apple: 50 
Diamond: 100")
  (bind _asbasic_widget_3 (Utilities|Casting|CastToBasicWidget (UserInterface|GetWidget (Variables|Default|GetBuyApple))))
  (Variables|/Script/UMG.TextBlock|SetText (Variables|/Game/UI/BasicWidget.BasicWidget_C|GetWidgetText _asbasic_widget_3) "Buy an Apple 
 |  
\\/")
  (bind _asbasic_widget_4 (Utilities|Casting|CastToBasicWidget (UserInterface|GetWidget (Variables|Default|GetBuyDiamond))))
  (Variables|/Script/UMG.TextBlock|SetText (Variables|/Game/UI/BasicWidget.BasicWidget_C|GetWidgetText _asbasic_widget_4) "Buy a Diamond 
 |  
\\/")
  (bind _asbasic_widget_5 (Utilities|Casting|CastToBasicWidget (UserInterface|GetWidget (Variables|Default|GetNomoney))))
  (Variables|/Script/UMG.TextBlock|SetText (Variables|/Game/UI/BasicWidget.BasicWidget_C|GetWidgetText _asbasic_widget_5) ""))
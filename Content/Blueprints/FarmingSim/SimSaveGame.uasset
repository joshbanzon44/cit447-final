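; SimSaveGame is a save game object for a farming sim that holds its economy and balance settings.
; A single SaveVariables function copies its inputs into matching member variables, covering harvest, growth, plots, NPCs, costs, taxes and watering can values.
; It is a plain data container with no load, slot-writing or validation logic.
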(fn SaveVariables
  (params (Input_GrainPerHarvest :type Integer) (Input_MoneyPerGrain :type Integer) (Input_GrowthPerSecond :type Float%20%28double-precision%29) (Input_PlotsAvailable :type Integer) (Input_MaxNPCs :type Integer) (Input_CostFirstNPC :type Integer) (Input_CostFirstPlot :type Integer) (Input_GrowthMultiplierNPC :type Float%20%28double-precision%29) (Input_WateringCanGrowthPercent :type Float%20%28double-precision%29) (Input_TaxPerIntervalPlot :type Integer) (Input_TaxPerIntervalNPC :type Integer) (Input_TaxInterval :type Float%20%28double-precision%29) (Input_CostFirstUpgrade :type Integer) (Input_MaxCanLevel :type Integer))
  (Variables|Default|SetGrainPerHarvest Input_GrainPerHarvest)
  (Variables|Default|SetMoneyPerGrain Input_MoneyPerGrain)
  (Variables|Default|SetGrowthPerSecond Input_GrowthPerSecond)
  (Variables|Default|SetPlotsAvailable Input_PlotsAvailable)
  (Variables|Default|SetMaxNpcs Input_MaxNPCs)
  (Variables|Default|SetCostFirstNPC Input_CostFirstNPC)
  (Variables|Default|SetCostFirstPlot Input_CostFirstPlot)
  (Variables|Default|SetGrowthMultiplierNPC Input_GrowthMultiplierNPC)
  (Variables|Default|SetWateringCanGrowthPercent Input_WateringCanGrowthPercent)
  (Variables|Default|SetTaxPerIntervalPlot Input_TaxPerIntervalPlot)
  (Variables|Default|SetTaxPerIntervalNPC Input_TaxPerIntervalNPC)
  (Variables|Default|SetTaxInterval Input_TaxInterval)
  (Variables|Default|SetCostFirstUpgrade Input_CostFirstUpgrade)
  (Variables|Default|SetMaxCanLevel Input_MaxCanLevel))
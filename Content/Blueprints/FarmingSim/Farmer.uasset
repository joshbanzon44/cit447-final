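; Farmer NPC for a farming sim that waters an assigned plot, refills its watering can and otherwise wanders.
; Every Tick, SetNewBehavior picks a state from interaction, plot assignment, can fuel and plot distance, and ChangeState swaps it on a state machine component with End/Start calls.
; BeginPlay sets the child-actor can's level from the save game.
; Hover toggles custom-depth highlighting, and Activate opens the farmer's UI with mouse control.
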(event EventBeginPlay
  (bind _returnvalue (SaveGame|LoadGamefromSlot "savegame"))
  (bind _assim_save_game (Utilities|Casting|CastToSimSaveGame _returnvalue))
  (Variables|Default|SetAs%20Sim%20Save%20Game _assim_save_game)
  (bind _aswatering_can (Utilities|Casting|CastToWateringCan (Variables|/Script/Engine.ChildActorComponent|GetChildActor (Variables|Default|GetWateringCan))))
  (bind _output_get (Variables|Default|SetWateringCanRef _aswatering_can))
  (Variables|/Game/Blueprints/FarmingSim/WateringCan.WateringCan_C|SetCanLevel _output_get (Variables|/Game/Blueprints/FarmingSim/SimSaveGame.SimSaveGame_C|GetGrowthMultiplierNPC (Variables|Default|GetAs%20Sim%20Save%20Game))))

(event EventHover
  (Rendering|SetRenderCustomDepth (Variables|Character|GetMesh) true))

(event EventTick
  (params (DeltaSeconds :type Float%20%28single-precision%29))
  (Default|FaceVelocity (Variables|Default|GetNavigationComp))
  (bind _newbehavior (CallFunction|SetNewBehavior (Variables|Default|GetCurrentStateENUM)))
  (CallFunction|ChangeState _newbehavior))

(event EventUnHover
  (Rendering|SetRenderCustomDepth (Variables|Character|GetMesh) false))

(event EventActivate
  (bind _returnvalue (UserInterface|CreateWidget "/Game/UI/FarmerInteractWidget.FarmerInteractWidget_C"))
  (Variables|Default|SetFarmerUI _returnvalue)
  (Variables|Default|SetInteracting true)
  (UserInterface|Viewport|AddtoViewport (Variables|Default|GetFarmerUI) 0)
  (bind _asgeneral_player_controller (Utilities|Casting|CastToGeneralPlayerController (Game|GetPlayerController 0)))
  (Default|EnableMouseControl _asgeneral_player_controller (Variables|Default|GetFarmerUI)))

(fn ConstructionScript)

(fn ChangeState
  (params (New%20State :type FarmerBehaviors%20Enum :default "NewEnumerator0"))
  (bind _statemachinecomponent (Variables|Default|GetStateMachineComponent))
  (if (Utilities|Enum|Equal(Enum) New%20State (Variables|Default|GetCurrentStateENUM))
    (return)
    (else
      (Utilities|FlowControl|Sequence
        (:then_0
          (Default|EndState (Variables|/Game/Blueprints/FarmingSim/States/StateMachineComponent.StateMachineComponent_C|GetCurrentState (Variables|Default|GetStateMachineComponent))))
        (:then_1
          (switch Utilities|FlowControl|Switch|SwitchonFarmerBehaviors New%20State
            (:NewEnumerator1
              (Default|ChangeState _statemachinecomponent "/Game/Blueprints/FarmingSim/States/WanderState.WanderState_C"))
            (:NewEnumerator2
              (Default|ChangeState _statemachinecomponent "/Game/Blueprints/FarmingSim/States/GetWaterState.GetWaterState_C"))
            (:NewEnumerator5
              (Default|ChangeState _statemachinecomponent "/Game/Blueprints/FarmingSim/States/GoToPlotState.GoToPlotState_C"))
            (:NewEnumerator6
              (Default|ChangeState _statemachinecomponent "/Game/Blueprints/FarmingSim/States/WateringState.WateringState_C"))
            (:NewEnumerator3
              (Default|ChangeState _statemachinecomponent "/Game/Blueprints/FarmingSim/States/InteractState.InteractState_C")))
          (return))
        (:then_2
          (Default|StartState (Variables|/Game/Blueprints/FarmingSim/States/StateMachineComponent.StateMachineComponent_C|GetCurrentState (Variables|Default|GetStateMachineComponent))))))))

(fn SetNewBehavior
  (params (CurrentBehavior :type FarmerBehaviors%20Enum :default "NewEnumerator0"))
  (bind _assignedplot (Variables|Default|GetAssignedPlot))
  (if (Variables|Default|GetInteracting)
    (return "NewEnumerator3")
    (else
      (Utilities|IsValid _assignedplot
        (:Is%20Valid
          (if (<= (Variables|/Game/Blueprints/FarmingSim/WateringCan.WateringCan_C|GetFuel (Variables|Default|GetWateringCanRef)) 0.0)
            (return "NewEnumerator2")
            (elif (<= (Math|Vector|Distance(Vector) (Transformation|GetActorLocation _assignedplot) (Transformation|GetActorLocation)) 2e+02)
              (return "NewEnumerator6")
              (else
                (return "NewEnumerator5")))))
        (:Is%20Not%20Valid
          (return "NewEnumerator1"))))))

(fn DestroyOwnedComponent
  (params (ComponentToDestory :type Actor%20Component%20Object%20Reference))
  (Components|DestroyComponent ComponentToDestory))
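; Farm plot actor in a farming sim that grows grass over time and yields grain to the player's FarmingStats when activated fully grown.
; Growth rate and harvest amount come from the save game; Tick adds the rate each frame, unscaled by delta time, updating a widget progress bar and three-stage grass height.
; UnlockPlot swaps materials and starts growth, hover toggles custom-depth highlighting, and player overlap only sets CanWater.
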(event EventBeginPlay
  (bind _asfarming_first_person_player_pawn (Utilities|Casting|CastToFarmingFirstPersonPlayerPawn (Game|Player|GetPlayerPawn 0)))
  (Variables|Default|SetPlayerRef _asfarming_first_person_player_pawn)
  (bind _returnvalue (SaveGame|LoadGamefromSlot "savegame"))
  (bind _assim_save_game (Utilities|Casting|CastToSimSaveGame _returnvalue))
  (bind _output_get (Variables|Default|SetSim%20Game%20Save _assim_save_game))
  (Variables|Default|SetGrowPercentPerSecond (Variables|/Game/Blueprints/FarmingSim/SimSaveGame.SimSaveGame_C|GetGrowthPerSecond _output_get))
  (bind _asprogress_bar (Utilities|Casting|CastToProgressBar (UserInterface|GetWidget (Variables|Default|GetPercentWidget))))
  (Variables|Default|SetProgressBar _asprogress_bar)
  (if (not (Variables|Default|GetLocked))
    (CallFunction|UnlockPlot)))

(event Collision|EventActorBeginOverlap
  (params (OtherActor :type Actor%20Object%20Reference))
  (if (== OtherActor (Variables|Default|GetPlayerRef))
    (Variables|Default|SetCanWater true)))

(event EventTick
  (params (DeltaSeconds :type Float%20%28single-precision%29))
  (bind _output_get (Variables|Default|SetPercentGrown (+ (Variables|Default|GetPercentGrown) (Variables|Default|GetGrowPercentPerSecond))))
  (CallFunction|UpdateBar _output_get)
  (CallFunction|ChangeHeight _output_get)
  (if (>= _output_get 1.0)
    (Actor|Tick|SetActorTickEnabled false)))

(event EventHover
  (Rendering|SetRenderCustomDepth (Variables|Default|GetPlotBase) true))

(event EventUnHover
  (Rendering|SetRenderCustomDepth (Variables|Default|GetDirt) false))

(event EventActivate
  (if (>= (Variables|Default|GetPercentGrown) 1.0)
    (Variables|Default|SetPercentGrown 0.0)
    (Actor|Tick|SetActorTickEnabled true)
    (Class|FarmingStatsComponent|ChangeGrain (Variables|/Game/Blueprints/Player/FarmingFirstPersonPlayerPawn.FarmingFirstPersonPlayerPawn_C|GetFarmingStats (Variables|Default|GetPlayerRef)) (Variables|/Game/Blueprints/FarmingSim/SimSaveGame.SimSaveGame_C|GetGrainPerHarvest (Variables|Default|GetSim%20Game%20Save)))
    (CallFunction|ChangeHeight 0.0)
    (CallFunction|UpdateBar 0.0)))

(event Collision|EventActorEndOverlap
  (params (OtherActor :type Actor%20Object%20Reference))
  (Variables|Default|SetCanWater false))

(fn ConstructionScript)

(fn UnlockPlot
  (Variables|Default|SetLocked false)
  (Rendering|Material|SetMaterial (Variables|Default|GetPlotBase) 0 "/Game/MundellsStarterContent/Materials/Wood.Wood")
  (Rendering|Material|SetMaterial (Variables|Default|GetDirt) 0 "/Game/MundellsStarterContent/Materials/Dirt.Dirt")
  (Actor|Tick|SetActorTickEnabled true)
  (Rendering|SetVisibility (Variables|Default|GetPercentWidget) true false))

(fn ChangeHeight
  (params (PercentDone :type Float%20%28double-precision%29))
  (if (>= PercentDone 1.0)
    (Transformation|SetRelativeScale3D (Variables|Default|GetGrass1) "1.500000,1.500000,20.000000")
    (elif (>= PercentDone 0.5)
      (Transformation|SetRelativeScale3D (Variables|Default|GetGrass1) "1.500000,1.500000,13.000000")
      (else
        (Transformation|SetRelativeScale3D (Variables|Default|GetGrass1) "1.500000,1.500000,5.000000")))))

(fn UpdateBar
  (params (NewPercent :type Float%20%28double-precision%29))
  (Progress|SetPercent (Variables|/Game/UI/ProgressBar.ProgressBar_C|GetProgressBar (Variables|Default|GetProgressBar)) NewPercent))
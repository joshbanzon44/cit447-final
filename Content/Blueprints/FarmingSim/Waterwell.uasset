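; Waterwell is a farming sim actor that refills the watering can of a player pawn or Farmer that overlaps it.
; It finds the can as the overlapping actor's first child actor and makes its meshes visible.
; The player gets a full refill immediately, with the HUD cooldown bar updated to match.
; A Farmer's can refills after a short delay, with no HUD update.
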(event EventBeginPlay)

(event Collision|EventActorBeginOverlap
  (params (OtherActor :type Actor%20Object%20Reference))
  (bind _asfarming_first_person_player_pawn (Utilities|Casting|CastToFarmingFirstPersonPlayerPawn OtherActor)
    (:then
      (bind _aswatering_can (Utilities|Casting|CastToWateringCan (Utilities|Array|Get(acopy) (Actor|GetAllChildActors _asfarming_first_person_player_pawn false))))
      (Rendering|SetVisibility (Variables|/Game/Blueprints/FarmingSim/WateringCan.WateringCan_C|GetCan _aswatering_can) true false)
      (bind _output_get (Variables|/Game/Blueprints/FarmingSim/WateringCan.WateringCan_C|SetFuel _aswatering_can 1e+02))
      (Progress|SetPercent (Variables|/Game/UI/FarmingPlayerHUD.FarmingPlayerHUD_C|GetCooldownBar (Variables|/Game/Blueprints/Player/FarmingFirstPersonPlayerPawn.FarmingFirstPersonPlayerPawn_C|GetHUD _asfarming_first_person_player_pawn)) (/ _output_get 1e+02)))
    (:CastFailed
      (bind _asfarmer (Utilities|Casting|CastToFarmer OtherActor))
      (bind _aswatering_can_2 (Utilities|Casting|CastToWateringCan (Utilities|Array|Get(acopy) (Actor|GetAllChildActors _asfarmer false))))
      (Rendering|SetVisibility (Variables|/Game/Blueprints/FarmingSim/WateringCan.WateringCan_C|GetCan _aswatering_can_2) true false)
      (Utilities|FlowControl|Delay 2.0)
      (Variables|/Game/Blueprints/FarmingSim/WateringCan.WateringCan_C|SetFuel _aswatering_can_2 1e+02))))

(event EventTick
  (params (DeltaSeconds :type Float%20%28single-precision%29)))

(fn ConstructionScript)
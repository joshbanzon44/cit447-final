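; Market is an interactable farming-sim world actor that opens a shop UI when activated.
; It creates the ShopUI widget on BeginPlay, and Activate adds it to the viewport and has the GeneralPlayerController enable mouse control for it.
; Hover and UnHover toggle custom depth rendering on its static mesh.
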(event EventBeginPlay
  (bind _returnvalue (UserInterface|CreateWidget "/Game/UI/ShopUI.ShopUI_C"))
  (Variables|Default|SetShopUI _returnvalue))

(event Collision|EventActorBeginOverlap
  (params (OtherActor :type Actor%20Object%20Reference)))

(event EventTick
  (params (DeltaSeconds :type Float%20%28single-precision%29)))

(event EventUnHover
  (Rendering|SetRenderCustomDepth (Variables|Default|GetStaticMesh) false))

(event EventActivate
  (UserInterface|Viewport|AddtoViewport (Variables|Default|GetShopUI) 0)
  (bind _asgeneral_player_controller (Utilities|Casting|CastToGeneralPlayerController (Game|GetPlayerController 0)))
  (Default|EnableMouseControl _asgeneral_player_controller (Variables|Default|GetShopUI)))

(event EventHover
  (Rendering|SetRenderCustomDepth (Variables|Default|GetStaticMesh) true))

(fn ConstructionScript)
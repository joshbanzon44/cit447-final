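; PasswordDoor is an interactable door actor that opens when the correct password is entered.
; Hover and UnHover toggle the mesh's custom depth rendering for highlighting.
; Activate shows an InputWidget through SimpleWidgetComp, passes it the door's Password and binds Open to its success event.
; Open simply destroys the actor rather than animating it.
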(event Custom|Open
  (Actor|DestroyActor))

(event EventBeginPlay)

(event Collision|EventActorBeginOverlap
  (params (OtherActor :type Actor%20Object%20Reference)))

(event EventTick
  (params (DeltaSeconds :type Float%20%28single-precision%29)))

(event EventHover
  (Rendering|SetRenderCustomDepth (Variables|Default|GetStaticMesh) true))

(event EventActivate
  (Default|Show (Variables|Default|GetSimpleWidgetComp) (Variables|Default|GetDisplayText))
  (bind _asinput_widget (Utilities|Casting|CastToInputWidget (Default|GetDisplayedWidget (Variables|Default|GetSimpleWidgetComp))))
  (Variables|/Game/UI/InputWidget.InputWidget_C|SetCorrectPassword _asinput_widget (Variables|Default|GetPassword))
  (EventDispatchers|BindEventtoPasswordSuccessEvent _asinput_widget (delegate Custom|Open)))

(event EventUnHover
  (Rendering|SetRenderCustomDepth (Variables|Default|GetStaticMesh) false))

(fn ConstructionScript)
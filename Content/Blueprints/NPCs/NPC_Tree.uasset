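; NPC_Tree is an interactable apple tree that pays the player money based on their farming level.
; Activate spawns a spark burst just below each of its three apples, then calls ChangeMoney on the first-person player pawn with its FarmingLevel.
; Hover and UnHover toggle custom depth rendering on the apples.
; The apples stay in place after activation, and the graph has no cooldown.
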(event EventActivate
  (Effects|SpawnEmitteratLocation "/Game/MundellsStarterContent/ParticleSystems/SparkBurst.SparkBurst" (- (Transformation|GetWorldLocation (Variables|Default|GetApple1)) "0.000000,0.000000,30.000000") "180.000000,0.000000,0.000000" "5.000000,5.000000,5.000000")
  (Effects|SpawnEmitteratLocation "/Game/MundellsStarterContent/ParticleSystems/SparkBurst.SparkBurst" (- (Transformation|GetWorldLocation (Variables|Default|GetApple2)) "0.000000,0.000000,30.000000") "180.000000,0.000000,0.000000" "5.000000,5.000000,5.000000")
  (Effects|SpawnEmitteratLocation "/Game/MundellsStarterContent/ParticleSystems/SparkBurst.SparkBurst" (- (Transformation|GetWorldLocation (Variables|Default|GetApple3)) "0.000000,0.000000,30.000000") "180.000000,0.000000,0.000000" "5.000000,5.000000,5.000000")
  (bind _asfirst_person_player_pawn (Utilities|Casting|CastToFirstPersonPlayerPawn (Game|GetPlayerCharacter 0)))
  (Default|ChangeMoney _asfirst_person_player_pawn (* (Variables|/Game/Blueprints/Player/FirstPersonPlayerPawn.FirstPersonPlayerPawn_C|GetFarmingLevel _asfirst_person_player_pawn) 1)))

(event EventUnHover
  (Rendering|SetRenderCustomDepth (Variables|Default|GetApple1) false))

(event EventHover
  (Rendering|SetRenderCustomDepth (Variables|Default|GetApple1) true))

(fn ConstructionScript)
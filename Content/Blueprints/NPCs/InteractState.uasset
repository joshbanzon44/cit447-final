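; NPC interact state, a state object whose owner is expected to be a ParentNPC.
; StartState calls the parent, sets the NPC's current state enum and rotates the NPC once to face player character 0.
; EndState only calls the parent and prints a debug string, as StartState also does; the Tick and BeginPlay events are disabled stubs.
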(event EventBeginPlay
  (|CallParentFunction) ; This node is disabled and will not be called.\nDrag off pins to build functionality.
)

(event EventTick
  (params (DeltaSeconds :type Float%20%28single-precision%29))
  (|CallParentFunction DeltaSeconds) ; This node is disabled and will not be called.\nDrag off pins to build functionality.
)

(fn StartState
  (|CallParentFunction)
  (Development|PrintString "interacting")
  (bind _asparent_npc (Utilities|Casting|CastToParentNPC (Components|GetOwner)))
  (Variables|/Game/Blueprints/NPCs/ParentNPC.ParentNPC_C|SetCurrentStateENUM _asparent_npc "NewEnumerator3")
  (Transformation|SetActorRotation _asparent_npc (Math|Rotator|FindLookatRotation (Transformation|GetActorLocation _asparent_npc) (Transformation|GetActorLocation (Game|GetPlayerCharacter 0)))))

(fn EndState
  (|CallParentFunction)
  (Development|PrintString "end interact state"))
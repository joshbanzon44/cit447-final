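; FollowState is an NPC state component that makes its owning ParentNPC follow the player character.
; StartState sets the NPC's state enum, raises a Following flag and turns it toward the player, while EndState clears the flag.
; Each tick rotates the NPC to face the player and issues an AI MoveTo with an acceptance radius, without checking the flag.
; An interpolated follow-behind movement is left unconnected.
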(event EventBeginPlay
  (|CallParentFunction) ; This node is disabled and will not be called.\nDrag off pins to build functionality.
)

(event EventTick
  (params (DeltaSeconds :type Float%20%28single-precision%29))
  (|CallParentFunction DeltaSeconds)
  (bind _asparent_npc (Utilities|Casting|CastToParentNPC (Components|GetOwner)))
  (Transformation|SetActorRotation _asparent_npc (Math|Rotator|FindLookatRotation (Transformation|GetActorLocation _asparent_npc) (Transformation|GetActorLocation (Game|GetPlayerCharacter 0))))
  (AI|AIMoveTo _asparent_npc "0, 0, 0" (Game|GetPlayerCharacter 0) 2.5e+02 false))

(fn StartState
  (|CallParentFunction)
  (Development|PrintString "IN Follow START")
  (bind _asparent_npc (Utilities|Casting|CastToParentNPC (Components|GetOwner)))
  (Variables|/Game/Blueprints/NPCs/ParentNPC.ParentNPC_C|SetCurrentStateENUM _asparent_npc "NewEnumerator4")
  (Variables|Default|SetFollowing true)
  (Transformation|SetActorRotation _asparent_npc (Math|Rotator|FindLookatRotation (Transformation|GetActorLocation _asparent_npc) (Transformation|GetActorLocation (Game|GetPlayerCharacter 0)))))

(fn EndState
  (|CallParentFunction)
  (Variables|Default|SetFollowing false))
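; NPC_Mine is an interactable mining rock that earns the player money each time it is activated.
; Activate spawns a small explosion effect midway between the two rock components, then adds money to the FirstPersonPlayerPawn in proportion to its MiningLevel.
; Hover and UnHover toggle custom depth rendering on both rocks as a highlight, and the rock is never destroyed or depleted here.
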(event EventBeginPlay)

(event Collision|EventActorBeginOverlap
  (params (OtherActor :type Actor%20Object%20Reference)))

(event EventTick
  (params (DeltaSeconds :type Float%20%28single-precision%29)))

(event EventActivate
  (Effects|SpawnEmitteratLocation "/Game/MundellsStarterContent/ParticleSystems/Explosion.Explosion" (/ (+ (Transformation|GetWorldLocation (Variables|Default|GetRockInteract2)) (Transformation|GetWorldLocation (Variables|Default|GetRockInteract))) 2.0) "0, 0, 0" "0.050000,0.050000,0.050000")
  (bind _asfirst_person_player_pawn (Utilities|Casting|CastToFirstPersonPlayerPawn (Game|GetPlayerCharacter 0)))
  (Default|ChangeMoney _asfirst_person_player_pawn (* (Variables|/Game/Blueprints/Player/FirstPersonPlayerPawn.FirstPersonPlayerPawn_C|GetMiningLevel _asfirst_person_player_pawn) 1)))

(event EventUnHover
  (Rendering|SetRenderCustomDepth (Variables|Default|GetRockInteract) false))

(event EventHover
  (Rendering|SetRenderCustomDepth (Variables|Default|GetRockInteract) true))

(fn ConstructionScript)
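; NPC_Apple is an apple pickup that NPCs consume on overlap, with a reaction that depends on their job.
; Overlapping a ParentNPC switches on its Job to show a popup line and adjust hunger, happiness and liking through StatsComp, with Farmers gaining most.
; Unemployed and Farmer NPCs also pay the player money scaled by MoneyLikeMultiplier, while Miners pay nothing.
; The apple then destroys itself.
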(event EventBeginPlay)

(event Collision|EventActorBeginOverlap
  (params (OtherActor :type Actor%20Object%20Reference))
  (bind _asparent_npc (Utilities|Casting|CastToParentNPC OtherActor))
  (switch Utilities|FlowControl|Switch|SwitchonNPCJobs (Variables|/Game/Blueprints/NPCs/ParentNPC.ParentNPC_C|GetJob _asparent_npc)
    (:NewEnumerator0
      (Default|ShowPopupWIdget _asparent_npc "An apple! YUM")
      (Default|ChangeStat (Variables|/Game/Blueprints/NPCs/ParentNPC.ParentNPC_C|GetStatsComp _asparent_npc) 0 10 0.0 10 0.1)
      (bind _asfirst_person_player_pawn (Utilities|Casting|CastToFirstPersonPlayerPawn (Game|GetPlayerCharacter 0)))
      (Default|ChangeMoney _asfirst_person_player_pawn (Math|Float|Truncate (* (Variables|/Game/Blueprints/NPCs/ParentNPC.ParentNPC_C|GetMoneyLikeMultiplier _asparent_npc) 5)))
      (Actor|DestroyActor))
    (:NewEnumerator1
      (Default|ShowPopupWIdget _asparent_npc "Apples for my farm!")
      (Default|ChangeStat (Variables|/Game/Blueprints/NPCs/ParentNPC.ParentNPC_C|GetStatsComp _asparent_npc) 0 10 0.0 20 0.2)
      (bind _asfirst_person_player_pawn_2 (Utilities|Casting|CastToFirstPersonPlayerPawn (Game|GetPlayerCharacter 0)))
      (Default|ChangeMoney _asfirst_person_player_pawn_2 (Math|Float|Truncate (* (Variables|/Game/Blueprints/NPCs/ParentNPC.ParentNPC_C|GetMoneyLikeMultiplier _asparent_npc) 10)))
      (Actor|DestroyActor))
    (:NewEnumerator2
      (Default|ShowPopupWIdget _asparent_npc "I dont really need this.")
      (Default|ChangeStat (Variables|/Game/Blueprints/NPCs/ParentNPC.ParentNPC_C|GetStatsComp _asparent_npc) 0 10 0.0 0 0.0)
      (Actor|DestroyActor))))

(event EventTick
  (params (DeltaSeconds :type Float%20%28single-precision%29)))

(fn ConstructionScript)
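; IdleState is the idle state in an NPC state machine, built on a parent state class with start, update and end functions.
; On start it calls the parent, prints a debug message, casts its owner to ParentNPC and sets that NPC's current state enum.
; Update and end only pass through to the parent, and BeginPlay and Tick are unused.
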(event EventBeginPlay
  (|CallParentFunction) ; This node is disabled and will not be called.\nDrag off pins to build functionality.
)

(event EventTick
  (params (DeltaSeconds :type Float%20%28single-precision%29))
  (|CallParentFunction DeltaSeconds) ; This node is disabled and will not be called.\nDrag off pins to build functionality.
)

(fn StartState
  (|CallParentFunction)
  (Development|PrintString "IN IDLE START")
  (bind _asparent_npc (Utilities|Casting|CastToParentNPC (Components|GetOwner)))
  (Variables|/Game/Blueprints/NPCs/ParentNPC.ParentNPC_C|SetCurrentStateENUM _asparent_npc "NewEnumerator1"))

(fn EndState
  (|CallParentFunction))

(fn UpdateState
  (params (InputState :type Base%20State%20Class%20Reference))
  (bind _new_state (|CallParentFunction InputState))
  (return _new_state))
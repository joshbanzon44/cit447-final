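; A3_NPC_Tutorial is a tutorial greeter actor that shows the assignment's welcome message and win goal.
; On BeginPlay it casts three widget components to BasicWidget, setting the title to the $10,000 goal text and blanking both guide labels.
; Any actor overlap destroys it, so the message disappears on first contact.
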(event EventBeginPlay
  (bind _asbasic_widget (Utilities|Casting|CastToBasicWidget (UserInterface|GetWidget (Variables|Default|GetTitle))))
  (Variables|/Script/UMG.TextBlock|SetText (Variables|/Game/UI/BasicWidget.BasicWidget_C|GetWidgetText _asbasic_widget) "Welcome to my Assignment 3! 
 
Get $10,000 to win!")
  (bind _asbasic_widget_2 (Utilities|Casting|CastToBasicWidget (UserInterface|GetWidget (Variables|Default|GetGuideLeft))))
  (Variables|/Script/UMG.TextBlock|SetText (Variables|/Game/UI/BasicWidget.BasicWidget_C|GetWidgetText _asbasic_widget_2) "")
  (bind _asbasic_widget_3 (Utilities|Casting|CastToBasicWidget (UserInterface|GetWidget (Variables|Default|GetGuideRight))))
  (Variables|/Script/UMG.TextBlock|SetText (Variables|/Game/UI/BasicWidget.BasicWidget_C|GetWidgetText _asbasic_widget_3) ""))

(event Collision|EventActorBeginOverlap
  (params (OtherActor :type Actor%20Object%20Reference))
  (Actor|DestroyActor))

(fn ConstructionScript)
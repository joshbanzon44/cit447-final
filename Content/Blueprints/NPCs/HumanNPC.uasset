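; HumanNPC is a human character that wanders around, facing its velocity, and tracks HP, hunger, age and happiness.
; Stat updates from StatsComp refresh its character widget and, once hunger reaches a threshold, send it via NavigationComp to the first fruit tree held by the game mode.
; Hover events toggle custom depth on the mesh, and Activate and Deactivate show or hide the widget.
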(event Custom|UpdateWidget
  (bind _statscomp (Variables|Default|GetStatsComp))
  (bind _hunger (Variables|/Game/Blueprints/Components/StatsComp.StatsComp_C|GetHunger _statscomp))
  (bind _ascharacter_widget (Utilities|Casting|CastToCharacterWidget (Default|GetDisplayedWidget (Variables|Default|GetSimpleWidgetComp)))
    (:then
      (Default|UpdateWidget _ascharacter_widget (Variables|/Game/Blueprints/Components/StatsComp.StatsComp_C|GetHP _statscomp) _hunger (Variables|/Game/Blueprints/Components/StatsComp.StatsComp_C|GetAge _statscomp) (Variables|/Game/Blueprints/Components/StatsComp.StatsComp_C|GetHappiness _statscomp)))
    (:CastFailed
      _))
  (if (>= _hunger (Variables|Default|GetFixHungerThreshold))
    (bind _asgeneral_game_mode (Utilities|Casting|CastToGeneralGameMode (Game|GetGameMode)))
    (Default|GotoLocation (Variables|Default|GetNavigationComp) (Transformation|GetActorLocation (Utilities|Array|Get(acopy) (Variables|/Game/Blueprints/GeneralGameMode.GeneralGameMode_C|GetFruitTrees _asgeneral_game_mode))))))

(event EventBeginPlay
  (Default|WanderAround (Variables|Default|GetNavigationComp) true)
  (EventDispatchers|BindEventtoOnStatUpdate (Variables|Default|GetStatsComp) (delegate Custom|UpdateWidget))
  (CallFunction|UpdateWidget))

(event EventActivate
  (Default|Show (Variables|Default|GetSimpleWidgetComp)))

(event EventDeactivate
  (Default|Hide (Variables|Default|GetSimpleWidgetComp)))

(event EventHover
  (Rendering|SetRenderCustomDepth (Variables|Default|GetStaticMesh) true))

(event EventTick
  (params (DeltaSeconds :type Float%20%28single-precision%29))
  (Default|FaceVelocity (Variables|Default|GetNavigationComp)))

(event EventUnHover
  (Rendering|SetRenderCustomDepth (Variables|Default|GetStaticMesh) false))

(fn ConstructionScript)
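; NPC_Diamond is a diamond item that reacts when an NPC overlaps it, with the outcome depending on that NPC's job.
; Unemployed and Miner NPCs show a delighted popup, gain happiness and liking, and pay the player money scaled by their MoneyLikeMultiplier, with Miners valuing it more.
; Farmers dismiss it, losing liking and paying nothing.
; The diamond destroys itself after these reactions.
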(event Collision|EventActorBeginOverlap
  (params (OtherActor :type Actor%20Object%20Reference))
  (bind _asparent_npc (Utilities|Casting|CastToParentNPC OtherActor))
  (switch Utilities|FlowControl|Switch|SwitchonNPCJobs (Variables|/Game/Blueprints/NPCs/ParentNPC.ParentNPC_C|GetJob _asparent_npc)
    (:NewEnumerator0
      (Default|ShowPopupWIdget _asparent_npc "hmm shiny")
      (Default|ChangeStat (Variables|/Game/Blueprints/NPCs/ParentNPC.ParentNPC_C|GetStatsComp _asparent_npc) 0 0 0.0 10 0.1)
      (bind _asfirst_person_player_pawn (Utilities|Casting|CastToFirstPersonPlayerPawn (Game|GetPlayerCharacter 0)))
      (Default|ChangeMoney _asfirst_person_player_pawn (Math|Float|Truncate (* (Variables|/Game/Blueprints/NPCs/ParentNPC.ParentNPC_C|GetMoneyLikeMultiplier _asparent_npc) 5)))
      (Actor|DestroyActor))
    (:NewEnumerator1
      (Default|ShowPopupWIdget _asparent_npc "Shiny but worthless")
      (Default|ChangeStat (Variables|/Game/Blueprints/NPCs/ParentNPC.ParentNPC_C|GetStatsComp _asparent_npc) 0 0 0.0 0 -0.1)
      (Actor|DestroyActor))
    (:NewEnumerator2
      (Default|ShowPopupWIdget _asparent_npc "OOOO SHINY")
      (Default|ChangeStat (Variables|/Game/Blueprints/NPCs/ParentNPC.ParentNPC_C|GetStatsComp _asparent_npc) 0 0 0.0 10 0.2)
      (bind _asfirst_person_player_pawn_2 (Utilities|Casting|CastToFirstPersonPlayerPawn (Game|GetPlayerCharacter 0)))
      (Default|ChangeMoney _asfirst_person_player_pawn_2 (Math|Float|Truncate (* (Variables|/Game/Blueprints/NPCs/ParentNPC.ParentNPC_C|GetMoneyLikeMultiplier _asparent_npc) 10)))
      (Actor|DestroyActor))))

(event EventTick
  (params (DeltaSeconds :type Float%20%28single-precision%29)))

(event EventBeginPlay)

(fn ConstructionScript)
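; Base NPC actor with stats, a job and a state machine for idle, wander, follow and interact behaviour.
; Stat updates refresh the info widget; full Liking doubles a money multiplier and, for Farmer or Miner, resets Liking and raises the player's matching skill.
; Tick turns the popup toward the player and evaluates state changes, which trigger speech popups.
; Hover toggles custom-depth highlighting; activation shows stats, pays the player and flags interaction.
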(event Custom|UpdateWidget
  (bind _statscomp (Variables|Default|GetStatsComp))
  (bind _asnpccontrol_widget (Utilities|Casting|CastToNPCControlWidget (Default|GetDisplayedWidget (Variables|Default|GetSimpleWidgetComp))))
  (Default|UpdateWidget _asnpccontrol_widget (Variables|/Game/Blueprints/Components/StatsComp.StatsComp_C|GetName _statscomp) (Variables|/Game/Blueprints/Components/StatsComp.StatsComp_C|GetHP _statscomp) (Variables|/Game/Blueprints/Components/StatsComp.StatsComp_C|GetHunger _statscomp) (Variables|/Game/Blueprints/Components/StatsComp.StatsComp_C|GetAge _statscomp) (Variables|/Game/Blueprints/Components/StatsComp.StatsComp_C|GetHappiness _statscomp) (Variables|/Game/Blueprints/Components/StatsComp.StatsComp_C|GetLiking _statscomp))
  (Utilities|FlowControl|Sequence
    (:then_0
      ;[1 1 1] Give more money as NPC likes the player more
      (if (>= (Variables|/Game/Blueprints/Components/StatsComp.StatsComp_C|GetLiking _statscomp) 1.0)
        (Variables|Default|SetMoneyLikeMultiplier (* (Variables|Default|GetMoneyLikeMultiplier) 2.0))))
    (:then_1
      (if (>= (Variables|/Game/Blueprints/Components/StatsComp.StatsComp_C|GetLiking (Variables|Default|GetStatsComp)) 1.0)
        (switch Utilities|FlowControl|Switch|SwitchonNPCJobs (Variables|Default|GetJob)
          (:NewEnumerator1
            (CallFunction|ShowStateWidget "I like you! Take this!")
            (Variables|/Game/Blueprints/Components/StatsComp.StatsComp_C|SetLiking (Variables|Default|GetStatsComp) 0.0)
            (bind _asfirst_person_player_pawn (Utilities|Casting|CastToFirstPersonPlayerPawn (Game|GetPlayerCharacter 0)))
            (Variables|/Game/Blueprints/Player/FirstPersonPlayerPawn.FirstPersonPlayerPawn_C|SetFarmingLevel _asfirst_person_player_pawn (+ (Variables|/Game/Blueprints/Player/FirstPersonPlayerPawn.FirstPersonPlayerPawn_C|GetFarmingLevel _asfirst_person_player_pawn) 1))
            (CallFunction|UpdateWidget))
          (:NewEnumerator2
            (CallFunction|ShowStateWidget "I like you! Take this!")
            (Variables|/Game/Blueprints/Components/StatsComp.StatsComp_C|SetLiking (Variables|Default|GetStatsComp) 0.0)
            (bind _asfirst_person_player_pawn_2 (Utilities|Casting|CastToFirstPersonPlayerPawn (Game|GetPlayerCharacter 0)))
            (Variables|/Game/Blueprints/Player/FirstPersonPlayerPawn.FirstPersonPlayerPawn_C|SetMiningLevel _asfirst_person_player_pawn_2 (+ (Variables|/Game/Blueprints/Player/FirstPersonPlayerPawn.FirstPersonPlayerPawn_C|GetMiningLevel _asfirst_person_player_pawn_2) 1))
            (CallFunction|UpdateWidget)))))))

(event Custom|ShowPopupWIdget
  (params (Popup%20Text :type Text))
  (bind _asbasic_widget (Utilities|Casting|CastToBasicWidget (UserInterface|GetWidget (Variables|Default|GetWidget))))
  (Variables|/Script/UMG.TextBlock|SetText (Variables|/Game/UI/BasicWidget.BasicWidget_C|GetWidgetText _asbasic_widget) Popup%20Text)
  (Rendering|SetVisibility (Variables|Default|GetWidget) true false)
  (Utilities|FlowControl|Delay 5.0)
  (Rendering|SetVisibility (Variables|Default|GetWidget) false false))

(event EventBeginPlay
  (EventDispatchers|BindEventtoOnStatUpdate (Variables|Default|GetStatsComp) (delegate Custom|UpdateWidget))
  (CallFunction|UpdateWidget))

(event EventHover
  (Rendering|SetRenderCustomDepth (Variables|Default|GetStaticMesh) true))

(event EventTick
  (params (DeltaSeconds :type Float%20%28single-precision%29))
  (Transformation|SetWorldRotation (Variables|Default|GetWidget) (Math|Rotator|FindLookatRotation (Transformation|GetActorLocation) (Transformation|GetActorLocation (Game|GetPlayerCharacter 0))) false false)
  (Default|FaceVelocity (Variables|Default|GetNavigationComp))
  (bind _new_behavior (CallFunction|SetNewBehavior (Variables|Default|GetCurrentStateENUM)))
  (CallFunction|ChangeState _new_behavior))

(event EventUnHover
  (Rendering|SetRenderCustomDepth (Variables|Default|GetStaticMesh) false))

(event EventActivate
  (Default|Show (Variables|Default|GetSimpleWidgetComp) (Variables|/Game/Blueprints/Components/StatsComp.StatsComp_C|GetName (Variables|Default|GetStatsComp)))
  (Variables|Default|SetInteracting true)
  (bind _asfirst_person_player_pawn (Utilities|Casting|CastToFirstPersonPlayerPawn (Game|GetPlayerCharacter 0)))
  (Default|ChangeMoney _asfirst_person_player_pawn 10))

(event EventDeactivate
  (Default|Hide (Variables|Default|GetSimpleWidgetComp)))

(fn ConstructionScript)

(fn DestoryOwnedComponent
  (params (CompToDestroy :type Actor%20Component%20Object%20Reference))
  (Components|DestroyComponent CompToDestroy))

(fn ChangeState
  (params (New%20State :type NPCStates%20Enum :default "NewEnumerator0"))
  (bind _statemachinecomponent (Variables|Default|GetStateMachineComponent))
  (if (Utilities|Enum|Equal(Enum) New%20State (Variables|Default|GetCurrentStateENUM))
    (return)
    (else
      (Development|PrintString "changing state")
      (Utilities|FlowControl|Sequence
        (:then_0
          (Default|EndState (Variables|/Game/Blueprints/FarmingSim/States/StateMachineComponent.StateMachineComponent_C|GetCurrentState (Variables|Default|GetStateMachineComponent))))
        (:then_1
          (switch Utilities|FlowControl|Switch|SwitchonNPCStates New%20State
            (:NewEnumerator1
              (Default|ChangeState _statemachinecomponent "/Game/Blueprints/NPCs/IdleState.IdleState_C"))
            (:NewEnumerator2
              (Default|ChangeState _statemachinecomponent "/Game/Blueprints/FarmingSim/States/WanderState.WanderState_C"))
            (:NewEnumerator3
              (Default|ChangeState _statemachinecomponent "/Game/Blueprints/NPCs/InteractState.InteractState_C"))
            (:NewEnumerator4
              (Default|ChangeState _statemachinecomponent "/Game/Blueprints/NPCs/FollowState.FollowState_C")))
          (CallFunction|ShowPopupWIdget (Utilities|Select :Index (Variables|Default|GetCurrentStateENUM) :NewEnumerator0 "NULL" :NewEnumerator1 "Imma sit here..." :NewEnumerator2 "Imma walk around" :NewEnumerator3 "Whats up bruh" :NewEnumerator4 "Im following u"))
          (return))
        (:then_2
          (Default|StartState (Variables|/Game/Blueprints/FarmingSim/States/StateMachineComponent.StateMachineComponent_C|GetCurrentState (Variables|Default|GetStateMachineComponent))))))))

(fn SetNewBehavior
  (params (Current%20Behavior :type NPCStates%20Enum :default "NewEnumerator0"))
  (if (Variables|Default|GetInteracting)
    (return "NewEnumerator3")
    (elif (Utilities|Enum|Equal(Enum) Current%20Behavior "NewEnumerator4")
      (return "NewEnumerator4")
      (elif (Utilities|Enum|Equal(Enum) Current%20Behavior "NewEnumerator1")
        (return "NewEnumerator1")
        (else
          (return "NewEnumerator2"))))))

(fn ShowStateWidget
  (params (StateText :type Text)))
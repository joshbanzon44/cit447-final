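; General player controller that installs the shared Enhanced Input mapping and handles level restart and quit; options and mode-switch inputs are stubs.
; Helper functions toggle the cursor, input mode and pawn input for UI use, respecting a default-cursor flag.
; SwitchPawns replaces the first-person or top-down pawn with the other at its location and yaw.
; BeginPlay calls an empty CreateDataMap, leaving the farming DataTable-to-map loop disconnected.
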(event Input|EnhancedActionEvents|EnhancedInputActionIA_Exit
  (params (ActionValue :type Boolean) (ElapsedSeconds :type Float%20%28double-precision%29) (TriggeredSeconds :type Float%20%28double-precision%29) (InputAction :type Input%20Action%20Object%20Reference :default "/Game/Input/IA_Exit.IA_Exit"))
  (Game|QuitGame 0 "Quit" false))

(event Input|EnhancedActionEvents|EnhancedInputActionIA_Options
  (params (ActionValue :type Boolean) (ElapsedSeconds :type Float%20%28double-precision%29) (TriggeredSeconds :type Float%20%28double-precision%29) (InputAction :type Input%20Action%20Object%20Reference :default "/Game/Input/IA_Options.IA_Options")))

(event Input|EnhancedActionEvents|EnhancedInputActionIA_Restart
  (params (ActionValue :type Boolean) (ElapsedSeconds :type Float%20%28double-precision%29) (TriggeredSeconds :type Float%20%28double-precision%29) (InputAction :type Input%20Action%20Object%20Reference :default "/Game/Input/IA_Restart.IA_Restart"))
  (bind _returnvalue (Game|GetCurrentLevelName true))
  (Game|OpenLevel(byName) (Utilities|String|StringToName _returnvalue)))

(event Input|EnhancedActionEvents|EnhancedInputActionIA_SwitchModes
  (params (ActionValue :type Boolean) (ElapsedSeconds :type Float%20%28double-precision%29) (TriggeredSeconds :type Float%20%28double-precision%29) (InputAction :type Input%20Action%20Object%20Reference :default "/Game/Input/IA_SwitchModes.IA_SwitchModes")))

(event EventBeginPlay
  (Input|AddMappingContext (PlayerController|LocalPlayerSubsystems|GetEnhancedInputLocalPlayerSubsystem) "/Game/Input/GeneralInputMapping.GeneralInputMapping" 0 "(bIgnoreAllPressedKeysUntilRelease=True,bForceImmediately=False,bNotifyUserSettings=False)")
  (CallFunction|CreateDataMap))

(fn ConstructionScript)

(fn EnableMouseControl
  (params (WidgetToFocus :type User%20Widget%20Object%20Reference))
  (bind _self self)
  (if (not (and (Variables|Default|GetbShowMouseCursor) (Variables|Default|GetDefaultShowMouse)))
    (Variables|Default|SetbShowMouseCursor true)
    (Input|SetInputModeGameandUI _self WidgetToFocus "DoNotLock" true true)
    (Input|DisableInput (Game|Player|GetPlayerPawn 0) _self)))

(fn DisableMouseControl
  (if (not (Variables|Default|GetDefaultShowMouse))
    (Variables|Default|SetbShowMouseCursor false)
    (Input|SetInputModeGameOnly (Game|GetPlayerController 0) true)
    (Input|EnableInput (Game|Player|GetPlayerPawn 0) 0)))

(fn SwitchPawns
  (bind _output_get (LocalVariables|SetOldPawn (Pawn|GetControlledPawn)))
  (Utilities|Casting|CastToFirstPersonPlayerPawn _output_get
    (:then
      (bind _returnvalue (Game|SpawnActorfromClass "/Game/Blueprints/Player/TopDownPlayerPawn.TopDownPlayerPawn_C" (Math|Transform|MakeTransform (.location (Transformation|GetActorTransform (LocalVariables|GetOldPawn))) (Math|Rotator|MakeRotator 0.0 0.0 (.yaw (.rotation (Transformation|GetActorTransform (LocalVariables|GetOldPawn))))) "1.000000,1.000000,1.000000") "Undefined" "MultiplyWithRoot" 0 0))
      (LocalVariables|SetNewPawn _returnvalue))
    (:CastFailed
      (Utilities|Casting|CastToTopDownPlayerPawn (LocalVariables|GetOldPawn))
      (bind _returnvalue_2 (Game|SpawnActorfromClass "/Game/Blueprints/Player/FirstPersonPlayerPawn.FirstPersonPlayerPawn_C" (Math|Transform|MakeTransform (.location (Transformation|GetActorTransform (LocalVariables|GetOldPawn))) (Math|Rotator|MakeRotator 0.0 0.0 (.yaw (.rotation (Transformation|GetActorTransform (LocalVariables|GetOldPawn))))) "1.000000,1.000000,1.000000") "Undefined" "MultiplyWithRoot" 0 0))
      (LocalVariables|SetNewPawn _returnvalue_2)))
  (Pawn|Possess (LocalVariables|GetNewPawn))
  (Actor|DestroyActor (LocalVariables|GetOldPawn)))

(fn CreateDataMap)
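; StatsComp is an actor component that tracks HP, Hunger, Age, Happiness and Liking for its owner.
; Its tick interval is set to UpdateInterval, and each tick shifts Hunger, Age and Happiness by per-update rates.
; ChangeStat applies amounts to all five stats at once.
; Both paths clamp stats at zero with no upper limit, then fire OnStatUpdate so listeners can react.
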(event EventBeginPlay
  (Class|ActorComponent|SetComponentTickInterval (Variables|Default|GetUpdateInterval)))

(event EventTick
  (params (DeltaSeconds :type Float%20%28single-precision%29))
  (Variables|Default|SetHunger (Math|Integer|Max(Integer) (+ (Variables|Default|GetHunger) (Variables|Default|GetHungerChangePerUpdate))))
  (Variables|Default|SetAge (Math|Float|Max(Float) (+ (Variables|Default|GetAge) (Variables|Default|GetAgeChangePerUpdate)) 0.0))
  (Variables|Default|SetHappiness (Math|Integer|Max(Integer) (+ (Variables|Default|GetHappiness) (Variables|Default|GetHappinessChangePerUpdate))))
  (Default|CallOnStatUpdate))

(fn ChangeStat
  (params (ChangeHPAmt :type Integer) (ChangeHungerAmt :type Integer) (ChangeAgeAmt :type Float%20%28double-precision%29) (ChangeHappinessAmt :type Integer) (ChangeLikingAmt :type Float%20%28double-precision%29))
  (Variables|Default|SetHP (Math|Integer|Max(Integer) (+ ChangeHPAmt (Variables|Default|GetHP))))
  (Variables|Default|SetHunger (Math|Integer|Max(Integer) (+ ChangeHungerAmt (Variables|Default|GetHunger))))
  (Variables|Default|SetAge (Math|Float|Max(Float) (+ ChangeAgeAmt (Variables|Default|GetAge)) 0.0))
  (Variables|Default|SetHappiness (Math|Integer|Max(Integer) (+ ChangeHappinessAmt (Variables|Default|GetHappiness))))
  (Variables|Default|SetLiking (Math|Float|Max(Float) (+ ChangeLikingAmt (Variables|Default|GetLiking)) 0.0))
  (Default|CallOnStatUpdate))
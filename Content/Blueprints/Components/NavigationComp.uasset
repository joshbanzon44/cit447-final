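; Navigation component that drives its owning Pawn through AI MoveTo, either wandering or heading to a given location.
; WanderAround picks a random reachable nearby point and, if looping, re-runs itself on a timer through WanderFunc.
; GoToLocation calls Stop to halt movement and clear that timer, then moves to the navmesh-projected point, printing failures.
; Successful moves call ReachedGoal, and a FaceVelocity helper turns the pawn toward its movement direction.
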(event Custom|GoToLocation
  (params (Location :type Vector))
  (CallFunction|Stop)
  (bind _movementresult (AI|AIMoveTo (Variables|Default|GetOwningPawn) (.ProjectedLocation (AI|Navigation|ProjectPointtoNavigation Location 0 0 "100.000000,100.000000,300.000000")) 0 1e+02 false)
    (:then
      (switch Utilities|FlowControl|Switch|SwitchonEPathFollowingResult _movementresult
        (:Blocked
          _)
        (:OffPath
          _)
        (:Aborted
          _)
        (:Invalid
          _))
      (Development|PrintString "Can't Get There!" true true "(R=1.000000,G=0.000000,B=0.000000,A=1.000000)" 5.0 :!label _label))
    (:OnSuccess
      (Default|CallReachedGoal))
    (:OnFail
      (goto _label))))

(event Custom|WanderAround
  (params (Loop :type Boolean))
  (Variables|Default|SetLoopCurrentAction Loop)
  (bind (_randomlocation _returnvalue) (CallFunction|GetRandomReachablePointinRadius (Transformation|GetActorLocation (Components|GetOwner)) 1e+03))
  (if _returnvalue
    (bind _movementresult (AI|AIMoveTo (Variables|Default|GetOwningPawn) _randomlocation 0 5.0 false)
      (:then
        (switch Utilities|FlowControl|Switch|SwitchonEPathFollowingResult _movementresult
          (:Success
            _)
          (:Blocked
            _)
          (:OffPath
            _)
          (:Aborted
            _)
          (:Invalid
            _)))
      (:OnSuccess
        (Default|CallReachedGoal))))
  (if (Variables|Default|GetLoopCurrentAction)
    (bind _returnvalue_2 (Utilities|Time|SetTimerbyFunctionName 0 "WanderFunc" 3.0))
    (Variables|Default|SetRepeatActionTimer _returnvalue_2)))

(event EventBeginPlay
  (bind _aspawn (Utilities|Casting|CastToPawn (Components|GetOwner)))
  (Variables|Default|SetOwningPawn _aspawn))

(fn GetRandomReachablePointinRadius
  (params (Origin :type Vector%20%28by%20ref%29) (Radius :type Float%20%28single-precision%29))
  (bind (_randomlocation _returnvalue) (AI|Navigation|GetRandomReachablePointinRadius Origin Radius 0 0))
  (return _randomlocation _returnvalue))

(fn Stop
  (Components|Movement|StopMovementImmediately (Pawn|GetMovementComponent (Variables|Default|GetOwningPawn)))
  (Utilities|Time|ClearandInvalidateTimerbyHandle (Variables|Default|GetRepeatActionTimer)))

(fn FaceVelocity
  (bind _owningpawn (Variables|Default|GetOwningPawn))
  (bind _returnvalue (Transformation|GetVelocity _owningpawn))
  (if (not (Math|Vector|VectorIsNearlyZero _returnvalue))
    (Transformation|SetActorRotation (Variables|Default|GetOwningPawn) (Math|Rotator|MakeRotfromX _returnvalue))))

(fn WanderFunc
  (CallFunction|WanderAround (Variables|Default|GetLoopCurrentAction)))
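; Component that shows, hides and swaps a single screen widget of a configurable class.
; Show lazily creates and caches the widget, adds it to the viewport and enables mouse control on GeneralPlayerController.
; A newly created NPCControlWidget also gets its name text from the initial text passed in.
; ChangeWidget discards the cached widget, sets the new class and re-shows it only if the old one was visible.
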(fn Show
  (params (InitialText :type Text))
  (Utilities|IsValid (Variables|Default|GetWidget)
    (:Is%20Valid
      (if (not (UserInterface|Viewport|IsinViewport (Variables|Default|GetWidget)))
        (UserInterface|Viewport|AddtoViewport (Variables|Default|GetWidget) 0 :!label _label)
        (bind _asgeneral_player_controller (Utilities|Casting|CastToGeneralPlayerController (Game|GetPlayerController 0)))
        (Default|EnableMouseControl _asgeneral_player_controller (Variables|Default|GetWidget))))
    (:Is%20Not%20Valid
      ;[1 1 1] Create for the first time
      (bind _returnvalue (UserInterface|CreateWidget (Variables|Default|GetWidgetClass)))
      (bind _output_get (Variables|Default|SetWidget _returnvalue))
      (bind _asnpccontrol_widget (Utilities|Casting|CastToNPCControlWidget _output_get)
        (:then
          (Variables|/Script/UMG.TextBlock|SetText (Variables|/Game/UI/NPCControlWidget.NPCControlWidget_C|GetTextName _asnpccontrol_widget) InitialText)
          (goto _label))
        (:CastFailed
          (goto _label))))))

(fn Hide
  (bind _widget (Variables|Default|GetWidget))
  (Utilities|IsValid _widget
    (:Is%20Valid
      (if (UserInterface|Viewport|IsinViewport _widget)
        (Widget|RemovefromParent _widget)))))

(fn GetDisplayedWidget
  (return (Variables|Default|GetWidget)))

(fn ChangeWidget
  (params (NewWidgetClass :type User%20Widget%20Class%20Reference) (NewInitialText :type Text))
  (LocalVariables|SetWasInViewport (UserInterface|Viewport|IsinViewport (Variables|Default|GetWidget)))
  (Widget|RemovefromParent (Variables|Default|GetWidget))
  (Variables|Default|SetWidgetClass NewWidgetClass)
  (Variables|Default|SetWidget 0)
  (if (LocalVariables|GetWasInViewport)
    (CallFunction|Show NewInitialText)))
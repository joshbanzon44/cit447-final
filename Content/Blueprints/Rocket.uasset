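; Rocket is an interactable actor that highlights on hover, then launches and explodes when activated.
; Hover and UnHover toggle custom depth rendering on its mesh parts.
; Activate attaches a fire emitter to a PhysicsThruster and switches the thruster on after a short delay.
; After a further delay it spawns an explosion at the rocket's location and destroys the actor.
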(event EventBeginPlay)

(event Collision|EventActorBeginOverlap
  (params (OtherActor :type Actor%20Object%20Reference)))

(event EventTick
  (params (DeltaSeconds :type Float%20%28single-precision%29)))

(event EventHover
  (Rendering|SetRenderCustomDepth (Variables|Default|Getrocket_Cylinder) true))

(event EventUnHover
  (Rendering|SetRenderCustomDepth (Variables|Default|Getrocket_Cylinder) false))

(event EventActivate
  (Effects|SpawnEmitterAttached "/Game/MundellsStarterContent/ParticleSystems/Fire.Fire" (Variables|Default|GetPhysicsThruster) "None" "0, 0, 0" "0, 0, 0" "2.000000,2.000000,2.000000")
  (Utilities|FlowControl|Delay 0.5)
  (Components|Activation|Activate (Variables|Default|GetPhysicsThruster) false)
  (Utilities|FlowControl|Delay 2.0)
  (Effects|SpawnEmitteratLocation "/Game/MundellsStarterContent/ParticleSystems/Explosion.Explosion" (Transformation|GetActorLocation))
  (Actor|DestroyActor))

(fn ConstructionScript)